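; Actor that spawns a performance-test camera and flies it along its spline path.
; On BeginPlay it spawns a PerfTestCamera_BP at its own transform and plays a timeline with its rate scaled by TimelineLength.
; Each update maps the timeline alpha to a distance along the spline, moving the camera there and facing it along the tangent.
; When the timeline finishes, it sets HasFinishedRoute on the camera.
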(event `self.ReceiveBeginPlay`
  (bind _returnvalue (`|SpawnActorFromClass` "/MemBenchmark/PerfTestCamera_BP.PerfTestCamera_BP_C" (`self.GetTransform` self) "AdjustIfPossibleButAlwaysSpawn" "MultiplyWithRoot" null null))
  (set `self.Camera` _returnvalue)
  (`TimelineComponent.SetPlayRate` (`self.Timeline`) (/ 1.0 (`self.TimelineLength`)))
  (`self.Play timeline`))

(event `Play timeline`
  (bind _spline (`self.Spline`))
  (bind (_direction _newtrack_0) (`Timeline|Timeline` :!via `PlayFromStart`)
    (:`Update`
      (bind _returnvalue (`KismetMathLibrary.Lerp` 0.0 (`SplineComponent.GetDistanceAlongSplineAtSplinePoint` _spline (- (`SplineComponent.GetNumberOfSplinePoints` _spline) 1)) _newtrack_0))
      (`self.K2_SetActorLocation` (`self.Camera`) (`SplineComponent.GetLocationAtDistanceAlongSpline` (`self.Spline`) _returnvalue "World") false false)
      (`self.K2_SetActorRotation` (`self.Camera`) (`KismetMathLibrary.Conv_VectorToRotator` (`SplineComponent.GetTangentAtDistanceAlongSpline` (`self.Spline`) _returnvalue "World")) false))
    (:`Finished`
      (set `PerfTestCamera.hasFinishedRoute` true (`self.Camera`)))))

(fn `UserConstructionScript`)